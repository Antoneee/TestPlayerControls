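; Quest giver logic that responds when the player interacts with its owning object or NPC.
; InteractWith asks the player's quest log component whether the configured quest is active.
; If not, DisplayQuest reads the quest's data table row and prints its name; otherwise a debug message reports it is already taken.
; Both branches return the owner's display name as the objective ID, and neither adds the quest to the log.
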(fn `DisplayQuest`
  (bind (_questdata_datatable _questdata_rowname) (break `DataTableRowHandle` (`self.QuestData`)))
  ;[1 1 1] Displays the quest name
  (bind _returnvalue (`|GetDataTableRow` _questdata_datatable _questdata_rowname)
    (:`then`
      (`KismetSystemLibrary.PrintString` (`KismetTextLibrary.Conv_TextToString` (`.QuestName_8_B1F695074F2A9A1A8106CCB9586ACBDB` (break `/Game/QuestSystem/S_QuestDetails` _returnvalue)))))))

(fn `InteractWith`
  (returns (ObjectiveID :type String))
  (bind (_questdata_datatable _questdata_rowname) (break `DataTableRowHandle` (`self.QuestData`)))
  (bind _returnvalue (`KismetSystemLibrary.GetDisplayName` (`self.GetOwner`)))
  ;[1 1 1] When the player interacts with a quest giver (object, NPC, etc.) return the objective ID of that quest giver
  (if (not (`/Game/QuestSystem/BP_QuestLogComponent.QueryActiveQuest` (`/Game/ThirdPerson/Blueprints/BP_ThirdPersonCharacter.BP_QuestLogComponent` (`/Game/CommonFuncitonLibrary.GetMyPlayerCharacter`)) _questdata_rowname))
    (`self.DisplayQuest`)
    (return _returnvalue)
    (else
      (`KismetSystemLibrary.PrintString` "Alredy on quest")
      (return _returnvalue))))