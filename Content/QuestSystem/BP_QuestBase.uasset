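; BP_QuestBase is a quest actor that tracks objective progress for the current stage of one quest.
; On BeginPlay it loads quest details from the QuestData table by QuestId and resets a map of objective IDs to progress counts.
; It binds to the player character's objective-ID event, incrementing matching objectives up to their target.
; When an objective completes, it shows a W_Quest_Notification widget with the description and count.
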(event `self.ReceiveBeginPlay`
  (`self.GetQuestDetails`)
  (add `/Game/ThirdPerson/Blueprints/BP_ThirdPersonCharacter.OnObjectiveIDCalled` (`/Game/CommonFuncitonLibrary.GetMyPlayerCharacter`) (`|CreateDelegate` :!event `On Objective ID Heard`)))

(fn `GetObjectiveDetailsByID`
  (params (ObjectiveID :type String))
  (returns (`Array Element` :type "/Game/QuestSystem/S_ObjectiveDetails Structure"))
  (for _array_element (`.Objectives_25_176A933C4FE4B231591AEFA576EF67D6` (break `/Game/QuestSystem/S_StageDetails` (`self.CurrentStageDetails`)))
    (if (`KismetStringLibrary.EqualEqual_StrStr` (`.ObjectiveID_26_7B274C1448542D31CA59D3BC8487808A` (break `/Game/QuestSystem/S_ObjectiveDetails` _array_element)) ObjectiveID)
      (return _array_element))))

(fn `GetQuestDetails`
  ;[1 1 1] Get the Quest Details by Quest ID and store the data in the QuestDetails variable
  (bind _returnvalue (`|GetDataTableRow` "/Game/QuestSystem/QuestData.QuestData" (`self.QuestId`))
    (:`then`
      (bind _output_get (set `self.QuestDetails` _returnvalue))
      ;[1 1 1] Since every quest has stages, we get the current stage based on CurrentStage index variable
      (bind _output_get_2 (set `self.CurrentStageDetails` (`|GetArrayItem` (`.QuestStages_14_214B79E94A1541D364F3739A746C00FF` (break `/Game/QuestSystem/S_QuestDetails` _output_get)) (`self.CurrentStage`))))
      ;[1 1 1] Since every stage has objectives, we populate the CurrentObjectiveProgress array with the Objective IDs of the current stage
      (`BlueprintMapLibrary.Map_Clear` (`self.CurrentObjectiveProgress`))
      (for _array_element (`.Objectives_25_176A933C4FE4B231591AEFA576EF67D6` (break `/Game/QuestSystem/S_StageDetails` _output_get_2))
        (`BlueprintMapLibrary.Map_Add` (`self.CurrentObjectiveProgress`) (`.ObjectiveID_26_7B274C1448542D31CA59D3BC8487808A` (break `/Game/QuestSystem/S_ObjectiveDetails` _array_element)))))))

(fn `isObjectiveComplete`
  (params (ObjectiveID :type String))
  (returns (IsComplete :type Boolean))
  (return (>= (`BlueprintMapLibrary.Map_Find` (`self.CurrentObjectiveProgress`) ObjectiveID) (`.ObjectiveTargetQuantity_20_C85726094E9480538FC15A8725FAAAFF` (break `/Game/QuestSystem/S_ObjectiveDetails` (`self.GetObjectiveDetailsByID` ObjectiveID))))))

(fn `On Objective ID Heard`
  (params (ObjectiveID :type String))
  (bind (_objectivename _objectivedescription _objectivetype _objectiveid _objectivetargetquantity) (break `/Game/QuestSystem/S_ObjectiveDetails` (`self.GetObjectiveDetailsByID` ObjectiveID)))
  (bind (_value _returnvalue) (`BlueprintMapLibrary.Map_Find` (`self.CurrentObjectiveProgress`) ObjectiveID))
  ;[1 1 1] When the player interacts with a quest object, it will check if the object is part of the current objective progress
  (if _returnvalue
    (if (< _value _objectivetargetquantity)
      ;[1 1 1] If the object is part of the objective progress, increment tthe progress by 1. Ex: Find object 0/1 -> Find object 1/1
      (`BlueprintMapLibrary.Map_Add` (`self.CurrentObjectiveProgress`) ObjectiveID (+ _value 1))
      (bind _iscomplete (`self.isObjectiveComplete` ObjectiveID))
      (if _iscomplete
        (bind _returnvalue_2 (`|CreateWidget` "/Game/QuestSystem/UI/W_Quest_Notification.W_Quest_Notification_C" null (`|FormatText` "{ObjectiveDescription} {CurrentObjectiveProgress}/{ObjectiveTargetQuantity}" _objectivedescription _value _objectivetargetquantity)))
        (`UserWidget.AddToViewport` _returnvalue_2 0)
        (return)
        (else
          (return))))
    (else
      (return))))

(fn `UserConstructionScript`)