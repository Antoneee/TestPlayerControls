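; BP_Door is an interactable tutorial exit door that sends the player to TestDesertMap when it is part of the active quest.
; Interact checks quest "10001" on the player's BP_QuestLogComponent; if active, it plays a sound, shows a WBP_Fade widget and opens the level after a short delay.
; A trigger volume shows or hides a text prompt as the third-person character enters or leaves.
; ReturnObjectiveID identifies the door as a quest objective.
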(event `/Game/I_InteractionInterface.Interact`
  (if (`/Game/QuestSystem/BP_QuestLogComponent.QueryActiveQuest` (`self.GetComponentByClass` (`GameplayStatics.GetPlayerCharacter` 0) "/Game/QuestSystem/BP_QuestLogComponent.BP_QuestLogComponent_C") "10001")
    (`KismetSystemLibrary.PrintString` "Object is part of the current active quest")
    (`GameplayStatics.PlaySound2D` "/Engine/VREditor/Sounds/UI/Enter_Play.Enter_Play" 1.0 1.0 0.0 null null)
    (bind _returnvalue (`|CreateWidget` "/Game/UI/WBP_Fade.WBP_Fade_C"))
    (`UserWidget.AddToViewport` _returnvalue 0)
    (`/Game/UI/WBP_Fade.FadeEvent` _returnvalue)
    (`KismetSystemLibrary.Delay` 1.0)
    (`GameplayStatics.OpenLevel` "TestDesertMap")
    (else
      (`KismetSystemLibrary.PrintString` "Object is not part of the current active quest"))))

(event `self.Trigger.OnComponentBeginOverlap`
  (params (OverlappedComponent :type "PrimitiveComponent Object Reference") (OtherActor :type "Actor Object Reference") (OtherComp :type "PrimitiveComponent Object Reference") (OtherBodyIndex :type Integer) (bFromSweep :type Boolean) (SweepResult :type "HitResult Structure (by ref)"))
  (cast `/Game/ThirdPerson/Blueprints/BP_ThirdPersonCharacter` OtherActor)
  (`SceneComponent.SetHiddenInGame` (`self.TextRender`) false false))

(event `self.Trigger.OnComponentEndOverlap`
  (params (OverlappedComponent :type "PrimitiveComponent Object Reference") (OtherActor :type "Actor Object Reference") (OtherComp :type "PrimitiveComponent Object Reference") (OtherBodyIndex :type Integer))
  (cast `/Game/ThirdPerson/Blueprints/BP_ThirdPersonCharacter` OtherActor)
  (`SceneComponent.SetHiddenInGame` (`self.TextRender`) true false))

(fn `Return Objective ID`
  (returns (`Objective ID` :type String))
  (return "tutorialExitDoor"))

(fn `UserConstructionScript`)